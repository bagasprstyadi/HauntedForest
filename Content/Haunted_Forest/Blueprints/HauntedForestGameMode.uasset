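; Game mode for the Haunted Forest game that brings up the pause menu and game-over screen.
; BeginPlay enables input from the first player controller so the Pause action reaches this Blueprint.
; Pause creates the PauseMenu widget, switches to game-and-UI input with a cursor and pauses the game, with IsScreenShown blocking repeat opens.
; HandleGameOver only creates the GameOver widget and adds it to the viewport.
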(event EventBeginPlay
  ;[1 1 1] Init
  (Input|EnableInput (Game|GetPlayerController 0)))

(event EventTick
  (params (DeltaSeconds :type Float%20%28single-precision%29)))

(event EventHandleGameOver
  (bind _returnvalue (UserInterface|CreateWidget "/Game/Haunted_Forest/UI/GameOver.GameOver_C"))
  (UserInterface|Viewport|AddtoViewport _returnvalue 0))

(event Input|ActionEvents|InputActionPause
  (params (Key :type Key%20Structure))
  (bind _returnvalue (Game|GetPlayerController 0))
  ;[1 1 1] Pause Menu
  (:Pressed
    (if (not (Variables|Default|GetisScreenShown))
      (bind _returnvalue_2 (UserInterface|CreateWidget "/Game/Haunted_Forest/UI/PauseMenu.PauseMenu_C"))
      (UserInterface|Viewport|AddtoViewport _returnvalue_2 0)
      (Input|SetInputModeGameandUI _returnvalue _returnvalue_2 "DoNotLock" true)
      (Variables|/Script/Engine.PlayerController|SetbShowMouseCursor _returnvalue true)
      (Variables|Default|SetisScreenShown true)
      (Game|SetGamePaused true))))

(fn ConstructionScript)