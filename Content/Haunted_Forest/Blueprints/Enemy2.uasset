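; Enemy2 is a patrolling ghost enemy for a 2D side-scroller that drains the player's stamina on contact.
; Tick drives movement along X, reversing speed and direction at the left and right boundaries.
; It swaps idle and move flipbooks by velocity and flips the sprite's X scale to face travel direction.
; Overlapping the player character deducts stamina and flags damage unless the player is invisible.
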(event Custom|UpdateAnimation
  ;[1 1 1] Handle Animation
  (Sprite|SetFlipbook (Variables|Default|GetSprite) (select (> (Math|Vector|VectorLength (Transformation|GetVelocity)) 0.0) "/Game/Haunted_Forest/Assets/Sprites/Enemy/ghost_move.ghost_move" "/Game/Haunted_Forest/Assets/Sprites/Enemy/ghost_idle.ghost_idle")))

(event Collision|EventActorBeginOverlap
  (params (OtherActor :type Actor%20Object%20Reference))
  ;[1 1 1] Damage to Player
  (bind _as2dside_scroller_character (Utilities|Casting|CastTo2DSideScrollerCharacter OtherActor))
  (if (not (Variables|/Game/Haunted_Forest/Blueprints/2DSideScrollerCharacter.2DSideScrollerCharacter_C|GetisInvisible _as2dside_scroller_character))
    (Variables|/Game/Haunted_Forest/Blueprints/2DSideScrollerCharacter.2DSideScrollerCharacter_C|Setstamina _as2dside_scroller_character (- (Variables|/Game/Haunted_Forest/Blueprints/2DSideScrollerCharacter.2DSideScrollerCharacter_C|Getstamina _as2dside_scroller_character) 3e+01))
    (Variables|/Game/Haunted_Forest/Blueprints/2DSideScrollerCharacter.2DSideScrollerCharacter_C|SetisDamaged _as2dside_scroller_character true)))

(event EventTick
  (params (DeltaSeconds :type Float%20%28single-precision%29))
  (bind _returnvalue (Transformation|GetActorLocation))
  (bind _x (Math|Vector|BreakVector _returnvalue))
  ;[1 1 1] Tick - Updates animation
  (Utilities|FlowControl|Sequence
    (:then_0
      (Pawn|Input|AddMovementInput "1.000000, 0, 0" (Variables|Default|Getmovement_speed) false)
      (Utilities|FlowControl|Sequence
        (:then_0
          (if (> _x (Variables|Default|GetRight_X_Axis_Boundary))
            (Variables|Default|Setmovement_speed (Variables|Default|Getmovement_left_speed))
            (Variables|Default|SetbisMovingRight false)))
        (:then_1
          (if (< _x (Variables|Default|GetLeft_X_Axis_Boundary))
            (Variables|Default|Setmovement_speed (Variables|Default|Getmovement_right_speed))
            (Variables|Default|SetbisMovingRight true)))))
    (:then_1
      (Utilities|FlowControl|Sequence
        (:then_0
          (CallFunction|UpdateAnimation)
          (Math|Float|CompareFloat (.X (Math|Vector|BreakVector (Variables|/Script/Engine.MovementComponent|GetVelocity (Pawn|GetMovementComponent)))) 0.0
            (:>
              (Transformation|SetWorldScale3D (Variables|Default|GetSprite) "1.000000,1.000000,1.000000" :!label _label))
            (:==
              (if (Variables|Default|GetbisMovingRight)
                (goto _label)
                (else
                  (Transformation|SetWorldScale3D (Variables|Default|GetSprite) "-1.000000,1.000000,1.000000" :!label _label_2))))
            (:<
              (goto _label_2))))))))

(event EventBeginPlay
  ;[1 1 1] Init Player
  (Class|ActorComponent|SetIsReplicated (Variables|Default|GetSprite) true)
  (bind _asplayer_stats_instance (Utilities|Casting|CastToPlayerStatsInstance (Game|GetGameInstance))))

(fn ConstructionScript)