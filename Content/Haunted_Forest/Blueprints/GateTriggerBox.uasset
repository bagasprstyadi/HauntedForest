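; GateTriggerBox is a trigger volume at a gate that controls whether the side-scroller player is allowed to win.
; Overlap begin and end events set InTrigger and share one branch that shows or hides a TextRender prompt and sets IsCanWin on the 2DSideScrollerCharacter.
; The overlapping actor is not checked; the branch always casts player pawn 0, so any actor entering or leaving toggles the state.
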(event EventBeginPlay)

(event Collision|EventActorBeginOverlap
  (params (OtherActor :type Actor%20Object%20Reference))
  (bind _returnvalue (Game|Player|GetPlayerPawn 0))
  (bind _textrender (Variables|Default|GetTextRender))
  (Variables|Default|SetinTrigger true)
  (if (Variables|Default|GetinTrigger)
    (Rendering|SetVisibility _textrender true false)
    (bind _as2dside_scroller_character (Utilities|Casting|CastTo2DSideScrollerCharacter _returnvalue))
    (Variables|/Game/Haunted_Forest/Blueprints/2DSideScrollerCharacter.2DSideScrollerCharacter_C|SetisCanWin _as2dside_scroller_character true)
    (else
      (Rendering|SetVisibility _textrender false false)
      (bind _as2dside_scroller_character_2 (Utilities|Casting|CastTo2DSideScrollerCharacter _returnvalue))
      (Variables|/Game/Haunted_Forest/Blueprints/2DSideScrollerCharacter.2DSideScrollerCharacter_C|SetisCanWin _as2dside_scroller_character_2 false))))

(event EventTick
  (params (DeltaSeconds :type Float%20%28single-precision%29)))

(event Collision|EventActorEndOverlap
  (params (OtherActor :type Actor%20Object%20Reference))
  (bind _returnvalue (Game|Player|GetPlayerPawn 0))
  (bind _textrender (Variables|Default|GetTextRender))
  (Variables|Default|SetinTrigger false)
  (if (Variables|Default|GetinTrigger)
    (Rendering|SetVisibility _textrender true false)
    (bind _as2dside_scroller_character (Utilities|Casting|CastTo2DSideScrollerCharacter _returnvalue))
    (Variables|/Game/Haunted_Forest/Blueprints/2DSideScrollerCharacter.2DSideScrollerCharacter_C|SetisCanWin _as2dside_scroller_character true)
    (else
      (Rendering|SetVisibility _textrender false false)
      (bind _as2dside_scroller_character_2 (Utilities|Casting|CastTo2DSideScrollerCharacter _returnvalue))
      (Variables|/Game/Haunted_Forest/Blueprints/2DSideScrollerCharacter.2DSideScrollerCharacter_C|SetisCanWin _as2dside_scroller_character_2 false))))

(fn ConstructionScript)