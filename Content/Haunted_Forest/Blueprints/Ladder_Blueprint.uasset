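; Ladder trigger actor that detects when the 2D side-scroller character enters or leaves its overlap area.
; Begin and end overlap set an InTrigger flag and share one branch that toggles a text render's visibility.
; The branch then fires the ButtonTrueLadder or ButtonFalseLadder dispatcher to signal the change; climbing itself is not handled here.
; The text is flipped on each overlap change rather than set explicitly.
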(event EventBeginPlay)

(event EventTick
  (params (DeltaSeconds :type Float%20%28single-precision%29)))

(event Collision|EventActorBeginOverlap
  (params (OtherActor :type Actor%20Object%20Reference))
  (if (== (Utilities|GetClass OtherActor) "/Game/Haunted_Forest/Blueprints/2DSideScrollerCharacter.2DSideScrollerCharacter_C")
    (Variables|Default|SetInTrigger true)
    (if (Variables|Default|GetInTrigger)
      (Rendering|ToggleVisibility (Variables|Default|GetTextRender) false)
      (Default|CallButtonTrueLadder)
      (else
        (Rendering|ToggleVisibility (Variables|Default|GetTextRender) false)
        (Default|CallButtonFalseLadder)))))

(event Collision|EventActorEndOverlap
  (params (OtherActor :type Actor%20Object%20Reference))
  (if (== (Utilities|GetClass OtherActor) "/Game/Haunted_Forest/Blueprints/2DSideScrollerCharacter.2DSideScrollerCharacter_C")
    (Variables|Default|SetInTrigger false)
    (if (Variables|Default|GetInTrigger)
      (Rendering|ToggleVisibility (Variables|Default|GetTextRender) false)
      (Default|CallButtonTrueLadder)
      (else
        (Rendering|ToggleVisibility (Variables|Default|GetTextRender) false)
        (Default|CallButtonFalseLadder)))))

(fn ConstructionScript)